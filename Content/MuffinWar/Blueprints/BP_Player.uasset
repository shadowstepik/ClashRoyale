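; BP_Player is a player actor for MuffinWar that sets up one team's base when play begins.
; It shows the mouse cursor, then spawns a team-assigned castle at an offset from its root, aligned to the camera's yaw.
; It spawns and stores right and left towers around the castle, flipping their world-space offsets by the sign of the castle's yaw so the layout mirrors for opposite-facing sides.
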(event EventBeginPlay
  (Variables|/Script/Engine.PlayerController|SetbShowMouseCursor (Game|GetPlayerController 0) true)
  (bind _returnvalue (Game|SpawnActorfromClass "/Game/Main/Building/BP_Castle.BP_Castle_C" (Math|Transform|MakeTransform (+ (Variables|Default|GetStartCastleOfCameraOffset) (Transformation|GetWorldLocation (Variables|Default|GetDefaultSceneRoot))) (Math|Rotator|MakeRotator 0.0 0.0 (.yaw (Transformation|GetWorldRotation (Variables|Default|GetCamera))))) "AlwaysSpawn" 0 (Variables|Default|GetTeam) self))
  (Variables|Default|SetMyCastle _returnvalue)
  (bind _returnvalue_2 (Game|SpawnActorfromClass "/Game/Main/Building/BP_Tower.BP_Tower_C" (Math|Transform|MakeTransform (+ (Transformation|GetActorLocation (Variables|Default|GetMyCastle)) (Math|Vector|MakeVector (* (Math|Float|SelectFloat 1.0 -1.0 (>= (.yaw (Transformation|GetActorRotation (Variables|Default|GetMyCastle))) 0.0)) (Variables|Default|GetTowerXOffset)) (* (Math|Float|SelectFloat 1.0 -1.0 (>= (.yaw (Transformation|GetActorRotation (Variables|Default|GetMyCastle))) 0.0)) (Variables|Default|GetTowerYOffset)) 0.0)) (Math|Rotator|MakeRotator 0.0 0.0 (.yaw (Transformation|GetActorRotation (Variables|Default|GetMyCastle))))) "AlwaysSpawn" 0 (Variables|Default|GetTeam) self))
  (Variables|Default|SetRightTower _returnvalue_2)
  (bind _returnvalue_3 (Game|SpawnActorfromClass "/Game/Main/Building/BP_Tower.BP_Tower_C" (Math|Transform|MakeTransform (+ (Transformation|GetActorLocation (Variables|Default|GetMyCastle)) (Math|Vector|MakeVector (* (Math|Float|SelectFloat 1.0 -1.0 (>= (.yaw (Transformation|GetActorRotation (Variables|Default|GetMyCastle))) 0.0)) (Variables|Default|GetTowerXOffset)) (* (* (Math|Float|SelectFloat 1.0 -1.0 (>= (.yaw (Transformation|GetActorRotation (Variables|Default|GetMyCastle))) 0.0)) (Variables|Default|GetTowerYOffset)) -1.0) 0.0)) (Math|Rotator|MakeRotator 0.0 0.0 (.yaw (Transformation|GetActorRotation (Variables|Default|GetMyCastle))))) "AlwaysSpawn" 0 (Variables|Default|GetTeam) self))
  (Variables|Default|SetLeftTower _returnvalue_3))

(fn ConstructionScript)