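; BP_StateComponent is an actor component in MuffinWar that holds a unit's state and its fullness and max fullness values.
; Add and remove functions adjust both values without clamping, and their RepNotify handlers broadcast a fullness-changed event.
; BPDead switches the unit state and broadcasts OnDead.
; Initialization in BeginPlay and owner-specific death logic (muffin hitbox disabling, castle game end) are left unconnected and never run.
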(event EventBeginPlay
  (|CallParentFunction))

(fn BPAddFullness
  (params (Value :type Float%20%28single-precision%29))
  (Variables|Default|SetBP_Fullness (+ (Variables|Default|GetBP_Fullness) Value)))

(fn BPRemoveFullness
  (params (Value :type Float%20%28single-precision%29))
  (Variables|Default|SetBP_Fullness (- (Variables|Default|GetBP_Fullness) Value)))

(fn BPAddMaxFullness
  (params (Value :type Float%20%28single-precision%29))
  (Variables|Default|SetBP_MaxFullness (+ (Variables|Default|GetBP_MaxFullness) Value)))

(fn BPRemoveMaxFullness
  (params (Value :type Float%20%28single-precision%29))
  (Variables|Default|SetBP_MaxFullness (- (Variables|Default|GetBP_MaxFullness) Value)))

(fn BPDead
  (Variables|Default|SetBP_UnitState "NewEnumerator2")
  (Default|CallBPonDead))

(fn BPonRepFullness
  (Default|CallBPonFullnessChanged))

(fn BPonRepMaxFullness
  (Default|CallBPonFullnessChanged))