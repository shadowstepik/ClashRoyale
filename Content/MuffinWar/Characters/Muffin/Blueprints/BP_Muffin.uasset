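; BP_Muffin is a team-based muffin combat unit with a fullness-based health model and a head-socket health widget.
; DoAttack toggles its hitbox, whose server-side overlaps damage enemy muffins or any base building.
; Hits shrink MaxFullness, killing a muffin once it would reach current Fullness, while eaten projectiles lower both values.
; Death disables the hitbox, stops AI logic and sets a short lifespan.
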(event OnComponentBeginOverlap(Hitbox)
  (params (OverlappedComponent :type Primitive%20Component%20Object%20Reference) (OtherActor :type Actor%20Object%20Reference) (OtherComp :type Primitive%20Component%20Object%20Reference) (OtherBodyIndex :type Integer) (bFromSweep :type Boolean) (SweepResult :type Hit%20Result%20Structure%20%28by%20ref%29))
  (Networking|SwitchHasAuthority
    (:Authority
      (bind _asbp_muffin (Utilities|Casting|CastToBP_Muffin OtherActor)
        (:then
          (if (Utilities|Enum|NotEqual(Enum) (Variables|BP_Muffin_C|GetTeam _asbp_muffin) (Variables|Default|GetTeam))
            (if (> (- (Variables|/Game/MuffinWar/Characters/Muffin/AI/StateComponent.StateComponent_C|GetMaxFullness (Variables|BP_Muffin_C|GetStateComponent _asbp_muffin)) (Variables|/Game/MuffinWar/Characters/Muffin/AI/StateComponent.StateComponent_C|GetDamage (Variables|Default|GetStateComponent))) (Variables|/Game/MuffinWar/Characters/Muffin/AI/StateComponent.StateComponent_C|GetFullness (Variables|BP_Muffin_C|GetStateComponent _asbp_muffin)))
              (CallFunction|ChangeFullness(OnServer) _asbp_muffin (Variables|/Game/MuffinWar/Characters/Muffin/AI/StateComponent.StateComponent_C|GetDamage (Variables|Default|GetStateComponent)))
              (else
                (CallFunction|OnDeath(OnServer) _asbp_muffin (Variables|/Game/MuffinWar/Characters/Muffin/AI/StateComponent.StateComponent_C|GetDamage (Variables|Default|GetStateComponent)))))))
        (:CastFailed
          (bind _asbp_base_building (Utilities|Casting|CastToBP_BaseBuilding OtherActor))
          (if (>= (- (Variables|/Game/MuffinWar/Characters/Muffin/AI/StateComponent.StateComponent_C|GetFullness (Variables|/Game/Main/Building/BP_BaseBuilding.BP_BaseBuilding_C|GetStateComponent _asbp_base_building)) (Variables|/Game/MuffinWar/Characters/Muffin/AI/StateComponent.StateComponent_C|GetDamage (Variables|Default|GetStateComponent))) 0.0)
            (Default|TakeDamage _asbp_base_building (Variables|/Game/MuffinWar/Characters/Muffin/AI/StateComponent.StateComponent_C|GetDamage (Variables|Default|GetStateComponent)))
            (else
              (Default|DestroyBuilding _asbp_base_building))))))))

(event Custom|OnDeath%28OnServer%29
  (params (Damage :type Float%20%28single-precision%29))
  (bind _self self)
  (bind _returnvalue (AI|GetAIController _self))
  (Variables|/Game/MuffinWar/Characters/Muffin/AI/StateComponent.StateComponent_C|SetFullness (Variables|Default|GetStateComponent) (- (Variables|/Game/MuffinWar/Characters/Muffin/AI/StateComponent.StateComponent_C|GetMaxFullness (Variables|Default|GetStateComponent)) Damage))
  (if (Utilities|Enum|NotEqual(Enum) (Variables|/Game/MuffinWar/Characters/Muffin/AI/StateComponent.StateComponent_C|GetUnitState (Variables|Default|GetStateComponent)) "NewEnumerator2")
    (Collision|SetCollisionEnabled (Variables|Default|GetHitbox) "NoCollision")
    (Variables|/Game/MuffinWar/Characters/Muffin/AI/StateComponent.StateComponent_C|SetUnitState (Variables|Default|GetStateComponent) "NewEnumerator2")
    (if (Utilities|IsValid _returnvalue)
      (AI|Logic|StopLogic (Variables|/Script/AIModule.AIController|GetBrainComponent _returnvalue) "")
      (Actor|SetLifeSpan 0.5))))

(event Custom|ChangeFullness%28OnServer%29
  (params (Damage :type Float%20%28single-precision%29))
  (bind _statecomponent (Variables|Default|GetStateComponent))
  (Variables|/Game/MuffinWar/Characters/Muffin/AI/StateComponent.StateComponent_C|SetMaxFullness (Variables|Default|GetStateComponent) (- (Variables|/Game/MuffinWar/Characters/Muffin/AI/StateComponent.StateComponent_C|GetMaxFullness (Variables|Default|GetStateComponent)) Damage))
  (bind _asw_unit_healt (Utilities|Casting|CastToW_UnitHealt (UserInterface|GetUserWidgetObject (Variables|Default|GetWidget))))
  (Default|UpdateHP _asw_unit_healt (Variables|/Game/MuffinWar/Characters/Muffin/AI/StateComponent.StateComponent_C|GetFullness _statecomponent) (Variables|/Game/MuffinWar/Characters/Muffin/AI/StateComponent.StateComponent_C|GetMaxFullness _statecomponent)))

(event Custom|EatProjectile%28OnServer%29
  (params (Fulling :type Float%20%28single-precision%29))
  (bind _statecomponent (Variables|Default|GetStateComponent))
  (bind _statecomponent_2 (Variables|Default|GetStateComponent))
  (Variables|/Game/MuffinWar/Characters/Muffin/AI/StateComponent.StateComponent_C|SetFullness _statecomponent (- (Variables|/Game/MuffinWar/Characters/Muffin/AI/StateComponent.StateComponent_C|GetFullness _statecomponent) (/ Fulling 2.0)))
  (Variables|/Game/MuffinWar/Characters/Muffin/AI/StateComponent.StateComponent_C|SetMaxFullness _statecomponent (- (Variables|/Game/MuffinWar/Characters/Muffin/AI/StateComponent.StateComponent_C|GetMaxFullness _statecomponent) (/ Fulling 2.0)))
  (bind _asw_unit_healt (Utilities|Casting|CastToW_UnitHealt (UserInterface|GetUserWidgetObject (Variables|Default|GetWidget))))
  (Default|UpdateHP _asw_unit_healt (Variables|/Game/MuffinWar/Characters/Muffin/AI/StateComponent.StateComponent_C|GetFullness _statecomponent_2) (Variables|/Game/MuffinWar/Characters/Muffin/AI/StateComponent.StateComponent_C|GetMaxFullness _statecomponent_2)))

(event EventBeginPlay
  (bind _statecomponent (Variables|Default|GetStateComponent))
  (Networking|SwitchHasAuthority
    (:Authority
      (Variables|/Game/MuffinWar/Characters/Muffin/AI/StateComponent.StateComponent_C|SetUnitState (Variables|Default|GetStateComponent) "NewEnumerator1")
      (Variables|/Game/MuffinWar/Characters/Muffin/AI/StateComponent.StateComponent_C|SetMaxFullness _statecomponent (Variables|/Game/MuffinWar/Characters/Muffin/AI/StateComponent.StateComponent_C|GetConstMaxFullness _statecomponent)))))

(fn ConstructionScript
  (Transformation|AttachComponentToComponent (Variables|Default|GetWidget) (Variables|Character|GetMesh) "headSocket" "SnapToTarget" "SnapToTarget" "SnapToTarget" true))

(fn DoAttack
  (params (IsAttacking :type Boolean))
  (bind _hitbox (Variables|Default|GetHitbox))
  (if IsAttacking
    (Collision|SetCollisionEnabled _hitbox "QueryOnly")
    (else
      (Collision|SetCollisionEnabled _hitbox "NoCollision")
      (Variables|/Game/MuffinWar/Characters/Muffin/AI/StateComponent.StateComponent_C|SetUnitState (Variables|Default|GetStateComponent) "NewEnumerator1"))))